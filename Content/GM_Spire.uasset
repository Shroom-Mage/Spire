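; GM_Spire is a match game mode that runs an Arcana card deck and its effects.
; On play start it creates the match display widget and links it to itself, and it shuffles the deck when a match begins.
; DrawCard constructs the chosen card's effect object from its class, records card and effect as active, and gives the effect a reference to the match.
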(event `self.ReceiveBeginPlay`
  (bind _returnvalue (`|CreateWidget` "/Game/Interface/WBP_MatchDisplay.WBP_MatchDisplay_C"))
  (bind _output_get (set `self.Match Display` _returnvalue))
  (`UserWidget.AddToViewport` _output_get 0)
  (set `/Game/Interface/WBP_MatchDisplay.Match` self _returnvalue))

(event `self.OnBeginMatch`
  (`KismetArrayLibrary.Array_Shuffle` (`self.ArcanaDeck`)))

(fn `DrawCard`
  (params (CardIndex :type Integer))
  (returns (DrawnArcana :type "ArcanaEffect Object Reference"))
  (bind _output (`|GetArrayItem` (`self.ArcanaDeck`) CardIndex))
  (bind _returnvalue (`|GenericCreateObject` (`ArcanaAsset.Effect` _output)))
  (`KismetArrayLibrary.Array_Add` (`self.ActiveArcana`) _output)
  (`KismetArrayLibrary.Array_Add` (`self.ActiveEffects`) _returnvalue)
  (set `ArcanaEffect.Match` self _returnvalue)
  (return _returnvalue))

(fn `UserConstructionScript`)