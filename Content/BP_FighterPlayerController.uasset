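; Player controller for a fighting game that routes player input to the fighter pawn it possesses.
; On possess it casts the pawn to FighterPawn and stores it as OwningFighter.
; The Move axis and the Jump, Evade, Normal, Special and Cancel presses each forward directly to a matching fighter function, leaving the action logic to the pawn.
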(event `self.ReceivePossess`
  (params (PossessedPawn :type "Pawn Object Reference"))
  (bind _asfighter_pawn (cast `FighterPawn` PossessedPawn))
  (set `self.OwningFighter` _asfighter_pawn))

(event `InputAxis|Move`
  (params (AxisValue :type "Float (single-precision)"))
  (`FighterPawn.Move` (`self.OwningFighter`) AxisValue))

(event `InputAction|Jump`
  (params (Key :type "Key Structure"))
  (:`Pressed`
    (`FighterPawn.Jump` (`self.OwningFighter`))))

(event `InputAction|Evade`
  (params (Key :type "Key Structure"))
  (:`Pressed`
    (`FighterPawn.Evade` (`self.OwningFighter`))))

(event `InputAction|Normal`
  (params (Key :type "Key Structure"))
  (:`Pressed`
    (`FighterPawn.Normal` (`self.OwningFighter`))))

(event `InputAction|Special`
  (params (Key :type "Key Structure"))
  (:`Pressed`
    (`FighterPawn.Special` (`self.OwningFighter`))))

(event `InputAction|Cancel`
  (params (Key :type "Key Structure"))
  (:`Pressed`
    (`FighterPawn.HardCancel` (`self.OwningFighter`))))

(fn `UserConstructionScript`)