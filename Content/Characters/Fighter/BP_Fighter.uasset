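; Fighter character Blueprint that leaves an afterimage continuing the interrupted state when a hard cancel occurs.
; On BeginPlay it spawns one owned BP_Afterimage at an out-of-the-way location with ticking disabled, then reuses it.
; OnHardCancel teleports it to the fighter, enables its tick, and passes it the canceled velocity and state.
; An unconnected node for copying StateTime to the afterimage never runs.
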(event `self.ReceiveBeginPlay`
  (bind _returnvalue (`|SpawnActorFromClass` "/Game/Characters/Fighter/BP_Afterimage.BP_Afterimage_C" (`KismetMathLibrary.MakeTransform` (0.0 4000.0 0.0)) "Undefined" "MultiplyWithRoot" self null))
  (bind _output_get (set `self.Afterimage` _returnvalue))
  (`self.SetActorTickEnabled` _output_get false)
  (`self.SetOwner` (`self.Afterimage`) self))

(event `self.OnHardCancel`
  (params (CanceledState :type "FighterStateAsset Object Reference") (CanceledVelocity :type "Vector2D Structure"))
  (bind _afterimage (`self.Afterimage`))
  (`self.K2_SetActorTransform` (`self.Afterimage`) (`self.GetTransform`) false true)
  (`self.SetActorTickEnabled` (`self.Afterimage`) true)
  (set `FighterPawn.Velocity` CanceledVelocity _afterimage)
  (`self.EnterState` _afterimage CanceledState "REPLACE" false))

(fn `UserConstructionScript`)